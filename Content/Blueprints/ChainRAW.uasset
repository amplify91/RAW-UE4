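; Chain weapon with a physics sphere head that the owning RAWCharacter holds at its right hand and launches along an aim vector.
; In flight, the sphere halts at chain length and then drops under gravity.
; A hit anchors it via physics constraints, tethering the character's capsule and disabling movement.
; Return breaks both constraints and restores walking; airborne launches are limited to one until the character walks again while holding it.
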(event `self.ReceiveBeginPlay`
  (set `self.isHeld` true)
  (bind _asrawcharacter (cast `/Game/Characters/RAW/RAWCharacter` (`self.GetOwner`)))
  (bind _output_get (set `self.RAWCharacterReference` _asrawcharacter))
  (`CableComponent.SetAttachEndTo` (`self.Chain`) _output_get "None"))

(event `self.ReceiveActorBeginOverlap`
  (params (OtherActor :type "Actor Object Reference")))

(event `self.ReceiveTick`
  (params (DeltaSeconds :type "Float (single-precision)"))
  (bind _sphere (`self.Sphere`))
  (bind _rawcharacterreference (`self.RAWCharacterReference`))
  (if (`self.isHeld`)
    (`self.K2_SetActorTransform` (`KismetMathLibrary.Conv_VectorToTransform` (`SceneComponent.GetSocketLocation` (`Character.Mesh` _rawcharacterreference) "hand_r")))
    (`PrimitiveComponent.SetEnableGravity` _sphere false)
    (set `self.ChainStopped` false)
    (if (`CharacterMovementComponent.IsWalking` (`Character.CharacterMovement` _rawcharacterreference))
      (set `self.isChainJumpAvailable` true))
    (elif (>= (`KismetMathLibrary.VSize` (- (`SceneComponent.K2_GetComponentLocation` (`self.Sphere`)) (`SceneComponent.K2_GetComponentLocation` (`Character.CapsuleComponent` _rawcharacterreference)))) (`self.ChainLength`))
      (if (`self.ChainStopped`)
        (if (not (`self.isAnchored`))
          (`PrimitiveComponent.SetEnableGravity` _sphere true))
        (else
          (`PrimitiveComponent.SetAllPhysicsLinearVelocity` _sphere (0.0 0.0 0.0) false)
          (set `self.ChainStopped` true))))))

(event `self.ReceiveHit`
  (params (MyComp :type "PrimitiveComponent Object Reference") (Other :type "Actor Object Reference") (OtherComp :type "PrimitiveComponent Object Reference") (bSelfMoved :type Boolean) (HitLocation :type "Vector Structure") (HitNormal :type "Vector Structure") (NormalImpulse :type "Vector Structure") (Hit :type "HitResult Structure (by ref)"))
  (if (not (`self.isHeld`))
    (set `self.isAnchored` true)
    (`PhysicsConstraintComponent.SetConstrainedComponents` (`self.AnchorConstraint`) MyComp "None" OtherComp "None")
    (`PhysicsConstraintComponent.SetConstrainedComponents` (`self.ChainConstraint`) (`self.Sphere`) "None" (`Character.CapsuleComponent` (`self.RAWCharacterReference`)) "None")
    (`CharacterMovementComponent.DisableMovement` (`Character.CharacterMovement` (`self.RAWCharacterReference`)))))

(fn `Launch`
  (params (AimVector :type "Vector Structure"))
  (if (`self.isLaunchAvailable`)
    (if (`NavMovementComponent.IsFalling` (`Character.CharacterMovement` (`self.RAWCharacterReference`)))
      (if (`self.isChainJumpAvailable`)
        (set `self.isLaunchAvailable` false :!label _label)
        (set `self.isChainJumpAvailable` false)
        (set `self.isHeld` false)
        (set `self.isLaunching` true)
        (`PrimitiveComponent.AddImpulse` (`self.Sphere`) (* AimVector (`self.LaunchVelocity`)) "None" true))
      (else
        (goto _label)))))

(fn `Return`
  (bind _rawcharacterreference (`self.RAWCharacterReference`))
  (set `self.isReturning` true)
  (set `self.isLaunching` false)
  (set `self.isHeld` true)
  (`PrimitiveComponent.SetAllPhysicsLinearVelocity` (`self.Sphere`) (0.0 0.0 0.0) false)
  (set `self.isReturning` false)
  (set `self.isAnchored` false)
  (`PhysicsConstraintComponent.BreakConstraint` (`self.ChainConstraint`))
  (`PhysicsConstraintComponent.BreakConstraint` (`self.AnchorConstraint`))
  (`PrimitiveComponent.SetSimulatePhysics` (`Character.CapsuleComponent` _rawcharacterreference) false)
  (`CharacterMovementComponent.SetMovementMode` (`Character.CharacterMovement` _rawcharacterreference) "MOVE_Walking" 0))

(fn `UserConstructionScript`)