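; AimCursor is an actor that shows a sphere as the player's aiming cursor in the XZ plane.
; On BeginPlay it caches the RAWCharacter and uses its MaxChainLength as the cursor radius.
; Gamepad aim axes past a deadzone write the character's AimVector and show the sphere, with a delayed hide.
; Tick places the sphere along AimVector from the pawn; a mouse-trace alternative sits behind a hardcoded false branch.
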(event `self.ReceiveActorBeginOverlap`
  (params (OtherActor :type "Actor Object Reference")))

(event `self.ReceiveBeginPlay`
  (bind _asrawcharacter (cast `/Game/Characters/RAW/RAWCharacter` (`Controller.K2_GetPawn` (`GameplayStatics.GetPlayerController` 0))))
  (bind _output_get (set `self.RAWCharacterReference` _asrawcharacter))
  (set `self.GamepadCursorRadius` (`/Game/Characters/RAW/RAWCharacter.MaxChainLength` _output_get)))

(event `self.ReceiveTick`
  (params (DeltaSeconds :type "Float (single-precision)"))
  (bind _returnvalue (`GameplayStatics.GetPlayerController` 0))
  (bind _sphere (`self.Sphere`))
  (if false
    (`SceneComponent.K2_SetWorldLocation` _sphere (`KismetMathLibrary.MakeVector` (.x (`.Location` (`GameplayStatics.BreakHitResult` (`PlayerController.GetHitResultUnderCursorByChannel` _returnvalue "TraceTypeQuery3" false)))) 0.0 (.z (`.Location` (`GameplayStatics.BreakHitResult` (`PlayerController.GetHitResultUnderCursorByChannel` _returnvalue "TraceTypeQuery3" false))))) false)
    (`SceneComponent.SetVisibility` _sphere true true)
    (else
      (`SceneComponent.K2_SetWorldLocation` _sphere (+ (`SceneComponent.K2_GetComponentLocation` (`self.K2_GetRootComponent` (`Controller.K2_GetPawn` _returnvalue))) (* (stale `InputAxis|AimRightGamepad` _output_get) (`self.GamepadCursorRadius`))) false))))

(event `InputAxis|AimRightGamepad`
  (params (AxisValue :type "Float (single-precision)"))
  (bind _sphere (`self.Sphere`))
  (bind _returnvalue (`KismetMathLibrary.MakeVector` AxisValue 0.0 (stale `InputAxis|AimUpGamepad` AxisValue)))
  (if (>= (`KismetMathLibrary.VSize` _returnvalue) 0.9) :!label _label
    (`SceneComponent.SetVisibility` _sphere true true)
    (bind _output_get (set `/Game/Characters/RAW/RAWCharacter.AimVector` _returnvalue (stale `self.ReceiveBeginPlay` _output_get)))
    (`KismetSystemLibrary.Delay` 2.0)
    (`SceneComponent.SetVisibility` _sphere false false)))

(event `InputAxis|AimUpGamepad`
  (params (AxisValue :type "Float (single-precision)"))
  (goto _label))

(fn `UserConstructionScript`)