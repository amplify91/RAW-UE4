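; Game mode that sets up the player's RAWCharacter and respawns it after it is destroyed.
; On BeginPlay and each respawn, it spawns an aim cursor and HUD widget, stores both on the character, and binds its destroyed event.
; That event waits briefly, calls OnDestroyedRaw on the old character, spawns and possesses a replacement, then reruns the setup.
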(event `Respawn`
  (bind _asrawcharacter (cast `/Game/Characters/RAW/RAWCharacter` (`GameplayStatics.GetPlayerCharacter` 0) :!label _label))
  (add `self.OnDestroyed` _asrawcharacter (delegate `OnDestroyed_Event_0`))
  (bind _returnvalue (`|SpawnActorFromClass` "/Game/Blueprints/AimCursor.AimCursor_C" (`self.SpawnTransform`) true))
  (set `/Game/Characters/RAW/RAWCharacter.AimCursorReference` _returnvalue _asrawcharacter)
  (bind _returnvalue_2 (`|CreateWidget` "/Game/Blueprints/HUD.HUD_C" (`GameplayStatics.GetPlayerController` 0)))
  (bind _output_get (set `/Game/Characters/RAW/RAWCharacter.HUD Reference` _returnvalue_2 _asrawcharacter))
  (`UserWidget.AddToViewport` _output_get 0))

(event `self.ReceiveBeginPlay`
  (goto _label))

(event `OnDestroyed_Event_0`
  (`KismetSystemLibrary.Delay` 1.0)
  (`/Game/Characters/RAW/RAWCharacter.OnDestroyedRaw` (stale `Respawn` _asrawcharacter))
  (bind _returnvalue (`|SpawnActorFromClass` "/Game/Characters/RAW/RAWCharacter.RAWCharacter_C" (`self.SpawnTransform`)))
  (`Controller.Possess` (`GameplayStatics.GetPlayerController` 0) _returnvalue)
  (`self.Respawn`))

(fn `UserConstructionScript`)